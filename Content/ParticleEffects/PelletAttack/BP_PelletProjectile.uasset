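; BP_PelletProjectile is a Niagara-driven homing pellet attack that damages the player's targeted boss.
; It registers itself as the Niagara export callback handler and sets the system's attraction point to the current target's location every tick.
; When particle data returns, it spawns an explosion at a particle position, damages the RBoss by particle size, plays impact sounds, prints boss health and destroys itself.
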(event `self.ReceiveBeginPlay`
  (`NiagaraComponent.SetVariableObject` (`self.Niagara`) "User.BP_PelletAttackCallbackHandler" self)
  (set `self.PlayerTargeting` (`self.GetComponentByClass` (`GameplayStatics.GetGameMode`) "/Script/GP4_Team7.RPlayerTargetingComponent")))

(event `self.ReceiveParticleData`
  (params (Data :type "Array of BasicParticleData Structure (by ref)") (NiagaraSystem :type "NiagaraSystem Object Reference"))
  (for _array_element Data
    _)
  (bind (_position _size) (break `BasicParticleData` _array_element))
  (`NiagaraFunctionLibrary.SpawnSystemAtLocation` "/Game/ParticleEffects/N_Explosion.N_Explosion" _position)
  (bind _asrboss (cast `RBoss` (`RPlayerTargetingComponent.GetCurrentTarget` (`self.PlayerTargeting`))))
  (`RBoss.TakeDamageR` _asrboss _size)
  (`KismetSystemLibrary.PrintString` (`KismetStringLibrary.Concat_StrStr` "BOSS HEALTH:" (`KismetStringLibrary.Conv_DoubleToString` (`RBoss.GetHealthR` _asrboss))) true true (struct :`G` 0.909657 :`B` 1.0 :`A` 1.0) 5.0)
  (bind _returnvalue (`self.K2_GetActorLocation` _asrboss))
  (`GameplayStatics.PlaySoundAtLocation` "/Game/StarterContent/Audio/Explosion01.Explosion01" _returnvalue (struct) 0.3 1.0 0.0 null null null)
  (`GameplayStatics.PlaySoundAtLocation` "/Game/Sound/SFX/SoundCues/CueBossGrunt.CueBossGrunt" _returnvalue (struct) 0.5 1.0 0.0 null null null)
  (`self.K2_DestroyActor`))

(event `self.ReceiveTick`
  (params (DeltaSeconds :type "Float (single-precision)"))
  (`NiagaraComponent.SetVariableVec3` (`self.Niagara`) "AttractionPoint" (`self.K2_GetActorLocation` (`RPlayerTargetingComponent.GetCurrentTarget` (`self.PlayerTargeting`)))))

(fn `UserConstructionScript`)