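; Hostile shockwave actor that spreads a ring across a scaled plane and damages the player pawn caught inside it.
; A fire event applies the spawn data, then a timeline grows the ring by driving width and inner radius on a dynamic material.
; The same values, scaled to world units, form a 2D distance band that triggers damage once.
; Height and speed multiplier are stored but do not affect the wave.
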(event `self.ReceiveBeginPlay`
  (bind _returnvalue (`PrimitiveComponent.CreateDynamicMaterialInstance` (`self.StaticMesh`) 0 "/Game/Blueprints/Hostiles/Shockwave/MI_Shockwave.MI_Shockwave" "None"))
  (set `self.Material Instance` _returnvalue)
  (add `self.FireShockwaveEvent` (delegate `FireEvent`))
  (bind _asbp_player_pawn_new (cast `/Game/Blueprints/Player/BP_PlayerPawn_New` (`Controller.K2_GetPawn` (`GameplayStatics.GetPlayerController` 0))))
  (set `self.Player Pawn` _asbp_player_pawn_new))

(event `FireEvent`
  (params (ShockwaveSpawnData :type "RShockwaveSpawnData Structure"))
  (bind _returnvalue_x (`KismetMathLibrary.BreakVector` (`SceneComponent.K2_GetComponentScale` (`self.StaticMesh`))))
  (`SceneComponent.SetWorldScale3D` (`self.StaticMesh`) (`KismetMathLibrary.MakeVector` ShockwaveSpawnData_Scale ShockwaveSpawnData_Scale ShockwaveSpawnData_Scale))
  (set `self.Shockwave Height` ShockwaveSpawnData_Height)
  (set `self.Shockwave Spawn Data Speed Multiplier` ShockwaveSpawnData_SpeedMultiplier)
  (bind _output_get (set `self.Width` (`KismetMathLibrary.MapRangeClamped` ShockwaveSpawnData_ZoneWidth 0.0 1.0 0.0 0.3)))
  (`KismetSystemLibrary.PrintString` (`KismetStringLibrary.Concat_StrStr` "Width" (`KismetStringLibrary.Conv_DoubleToString` _output_get)))
  ;[1 1 1] The plane mesh is 100x100 units
  (set `self.ScaleMultiplier` (* _returnvalue_x 100.0))
  (bind _returnvalue (`MaterialInstanceDynamic.K2_GetScalarParameterValue` (`self.Material Instance`) "OuterLimit"))
  (set `self.OuterLimit` _returnvalue)
  (bind (_direction _deltatime) (`Timeline|Spread Circle`)
    (:`Update`
      (bind _output_get_2 (set `self.Radius Inner` _deltatime))
      (if (< _output_get_2 (`self.OuterLimit`))
        (`|ExecutionSequence`
          (:`then_0`
            (`MaterialInstanceDynamic.SetScalarParameterValue` (`self.Material Instance`) "Width" (`self.Width`))
            (`MaterialInstanceDynamic.SetScalarParameterValue` (`self.Material Instance`) "InnerRadius" (`self.Radius Inner`)))
          (:`then_1`
            (set `self.Outer Radius` (* (+ (`self.Radius Inner`) (`self.Width`)) (`self.ScaleMultiplier`)))
            (set `self.Inner Radius` (* (`self.Radius Inner`) (`self.ScaleMultiplier`))))
          (:`then_2`
            (bind _did_hit (`self.Check If Shockwave Hit Player` (`self.K2_GetActorLocation` (`self.Player Pawn`))))
            (if _did_hit
              (`/Engine/EditorBlueprintResources/StandardMacros.DoOnce` false
                (:`Completed`
                  (`RPlayerPawn.GetDamaged` (`self.Player Pawn`))
                  (`self.SetLifeSpan` 10.0))))))))
    (:`Finished`
      (`self.K2_DestroyActor`))))

(fn `Check If Shockwave Hit Player`
  (params (`Player World Location` :type "Vector Structure"))
  (returns (`Did Hit` :type Boolean))
  (locals (PlayerLoc :type "Vector Structure"))
  (bind _output_get (set `local.PlayerLoc` `Player World Location`))
  (bind _returnvalue (`self.Get 2D Distance to Player` _output_get))
  (return (and (< (`self.Inner Radius`) _returnvalue) (> (`self.Outer Radius`) _returnvalue) true)))

(fn `Get 2D Distance to Player`
  (params (PlayerLocation :type "Vector Structure"))
  (returns (ReturnValue :type "Float (double-precision)"))
  (return (`KismetMathLibrary.Distance2D` (`KismetMathLibrary.Conv_VectorToVector2D` (`self.K2_GetActorLocation`)) (`KismetMathLibrary.Conv_VectorToVector2D` PlayerLocation))))

(fn `UserConstructionScript`)