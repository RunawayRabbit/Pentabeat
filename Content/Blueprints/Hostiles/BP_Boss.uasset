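; Boss hostile whose attacks and movement are driven by music events from the game mode's music manager.
; Each played note's track selects a channel entry, which decides whether to fire a projectile or shockwave and whether to update movement.
; Note panning feeds the projectile data and sets movement direction and speed scale.
; It starts stationary, and its bound death handler is empty, with the completed-level screen code left disconnected.
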(event `self.ReceiveBeginPlay`
  (`|ExecutionSequence`
    (:`then_0`
      (`self.UpdateMovement` (make `RBossMovementData` 0.0)))
    (:`then_1`
      (bind _asrgame_mode_base (cast `RGameModeBase` (`GameplayStatics.GetGameMode`)))
      (set `self.MusicManager` (`self.GetComponentByClass` _asrgame_mode_base "/Script/GP4_Team7.RMusicManager"))
      (add `self.OnBossDeath` (delegate `OnBossDeathEvent`))
      (add `RMusicManager.MusicEvent` (`self.MusicManager`) (delegate `OnMusicEvent`)))))

(event `OnMusicEvent`
  (params (MusicEventInfo :type "MusicEventInfo Structure"))
  (bind (_spawn_type _move_type) (`self.Parse Music Info` MusicEventInfo))
  (`|ExecutionSequence`
    (:`then_0`
      (switch `ERUpdateMovement` _move_type
        (:`Update`
          (`self.UpdateMovement` (`self.Selected Movement Data`)))))
    (:`then_1`
      (switch `ERBossSpawnType` _spawn_type
        (:`Projectile`
          (`self.FireProjectile` (`self.Selected Projectile Data`)))
        (:`Shockwave`
          (`self.FireShockwave` (make `RShockwaveSpawnData` "/Game/Blueprints/Hostiles/Shockwave/BP_Shockwave.BP_Shockwave_C" 0.02 10.0 1.0 -79.0 100.0)))))))

(event `OnBossDeathEvent`
  ;[1 1 1] Display win screen
)

(fn `Parse Music Info`
  (params (`Music Event Info` :type "MusicEventInfo Structure"))
  (returns (`Spawn Type` :type "ERBossSpawnType Enum") (`Move Type` :type "ERUpdateMovement Enum"))
  (locals (PanningPercentage :type "Float (double-precision)"))
  (bind (_type _track _panning) (break `MusicEventInfo` `Music Event Info`))
  (bind _channel_projectiles (`self.Channel Projectiles`))
  (bind _returnvalue (`KismetMathLibrary.Conv_ByteToInt` _track))
  (bind _output (`|GetArrayItem` _channel_projectiles _returnvalue))
  (bind _movementtype (`RProjectileDefinition.MovementType` _output))
  (if (`|EnumEquality` _type "NotePlayed")
    (set `local.PanningPercentage` _panning)
    (if (< _returnvalue (`KismetArrayLibrary.Array_Length` _channel_projectiles))
      (`|ExecutionSequence`
        (:`then_0`
          (bind _output_get (set `self.Selected Projectile Data` (`RProjectileDefinition.ProjectileSpawnData` _output)))
          (setmembers `RProjectileSpawnData` :`StructRef` _output_get :`PanningPercentage` (`local.PanningPercentage`)))
        (:`then_1`
          (switch `ERUpdateMovement` _movementtype
            (:`Update`
              (bind _output_get_2 (set `self.Selected Movement Data` (`RProjectileDefinition.BossMovementData` _output)))
              (bind _structout (setmembers `RBossMovementData` :`StructRef` _output_get_2 :`Speed` (* (`.Speed` (break `RBossMovementData` _output_get_2)) (* 10 (`KismetMathLibrary.Abs` (`local.PanningPercentage`)))) :`MovementDirection` (select `bool` (>= (`local.PanningPercentage`) 0.0) :`false` "CounterClockwise" :`true` "Clockwise" :!type "ERMovementDirection Enum"))))))
        (:`then_2`
          (return (`RProjectileDefinition.ProjectileType` _output) _movementtype))))
    (else
      (return "None" "KeepCurrent"))))

(fn `UserConstructionScript`)