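; BP_WeirdBossThing is a hostile boss whose fight follows the sections of a song through marker events.
; At Verse 2 and Outro it checks its health and sends the music manager back to an earlier chorus while health remains at or above a threshold.
; At End, zero health shows the completed level screen once.
; A debug key bound on BeginPlay jumps straight to the second chorus.
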(event `self.ProcessMarker`
  (params (MarkerText :type String) (Manager :type "RMusicManager Object Reference"))
  (bind _returnvalue (`self.GetHealthR`))
  (switch `string` MarkerText
    (:`Verse 2`
      (if (>= _returnvalue 50.0)
        (`RMusicManager.GoBackToMarker` Manager "Chorus 1")))
    (:`Outro`
      (if (>= _returnvalue 0.0)
        (`RMusicManager.GoBackToMarker` Manager "Chorus 2")))
    (:`End`
      (if (<= _returnvalue 0.0)
        (`/Engine/EditorBlueprintResources/StandardMacros.DoOnce` false
          (:`Completed`
            (bind _returnvalue_2 (`|CreateWidget` "/Game/Blueprints/UI/BP_CompletedLevelScreen.BP_CompletedLevelScreen_C"))
            (`UserWidget.AddToViewport` _returnvalue_2 0)))))))

(event `self.ReceiveBeginPlay`
  ;[0.284 0.2499 1] Debug Junk
  (`parent.ReceiveBeginPlay`)
  (`self.EnableInput` (`GameplayStatics.GetPlayerController` 0)))

(event `InputAction|HenrikDebugKey`
  (params (Key :type "Key Structure"))
  ;[0.284 0.2499 1] Debug Junk
  (:`Pressed`
    (`RMusicManager.GoBackToMarker` (stale `self.ProcessMarker` Manager) "Chorus 2")))

(fn `UserConstructionScript`)