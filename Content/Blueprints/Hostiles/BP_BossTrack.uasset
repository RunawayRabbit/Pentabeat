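; BP_BossTrack is a spline-based track actor, named for bosses, that pairs each spline point with an entry in the SplinePointDatas array.
; The Construction Script adds default entries or removes trailing ones until the array length matches the spline's point count, using two helper checks.
; It has no runtime logic; its event graph holds only disabled placeholder events.
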(fn `Is Array Too Big?`
  (returns (IsTooBig :type Boolean))
  (return (> (`KismetArrayLibrary.Array_Length` (`self.SplinePointDatas`)) (`SplineComponent.GetNumberOfSplinePoints` (`self.SplineComponent`)))))

(fn `Is Array Too Small?`
  (returns (IsTooSmall :type Boolean))
  (return (> (`SplineComponent.GetNumberOfSplinePoints` (`self.SplineComponent`)) (`KismetArrayLibrary.Array_Length` (`self.SplinePointDatas`)))))

(fn `UserConstructionScript`
  (locals (SplinePoints :type Integer :default 0))
  (bind _splinepointdatas (`self.SplinePointDatas`))
  (`|ExecutionSequence`
    (:`then_0`
      (while (`self.Is Array Too Small?`)
        (`KismetArrayLibrary.Array_Add` (`self.SplinePointDatas`))))
    (:`then_1`
      (while (`self.Is Array Too Big?`)
        (`KismetArrayLibrary.Array_Remove` _splinepointdatas (`KismetArrayLibrary.Array_LastIndex` _splinepointdatas))))))