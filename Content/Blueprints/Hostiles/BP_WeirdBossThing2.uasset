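; Boss hostile that steers marker-based playback, apparently a song, according to its remaining health.
; ProcessMarker skips from Verse 2 or 3 to the outro once health is low, and loops from the outro back to verse 1 while it is higher.
; At Endbit it repeats the outro while any health remains, otherwise it shows the level-completed screen once.
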(event `self.ProcessMarker`
  (params (MarkerText :type String) (Manager :type "RMusicManager Object Reference"))
  (bind _returnvalue (> (`self.GetHealthR`) 5.0))
  (switch `string` MarkerText
    (:`verse 2`
      (if (not _returnvalue) :!label _label
        (`RMusicManager.GoBackToMarker` Manager "outro")))
    (:`verse 3`
      (goto _label))
    (:`outro`
      (if _returnvalue
        (`RMusicManager.GoBackToMarker` Manager "verse 1")))
    (:`endbit`
      (if (> (`self.GetHealthR`) 0.0)
        (`RMusicManager.GoBackToMarker` Manager "outro")
        (else
          (`/Engine/EditorBlueprintResources/StandardMacros.DoOnce` false
            (:`Completed`
              (bind _returnvalue_2 (`|CreateWidget` "/Game/Blueprints/UI/BP_CompletedLevelScreen.BP_CompletedLevelScreen_C"))
              (`UserWidget.AddToViewport` _returnvalue_2 0))))))))

(fn `UserConstructionScript`)