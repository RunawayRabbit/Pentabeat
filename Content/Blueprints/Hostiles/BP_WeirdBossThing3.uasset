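; Boss Blueprint that ties progress through its music track to its remaining health.
; On each music-style marker it receives, it checks health against a descending threshold and sends the marker Manager back to an earlier chorus while health is still above it.
; The Outro repeats from the last chorus until health is depleted, and the End marker shows the level-completed screen once.
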(event `self.ProcessMarker`
  (params (MarkerText :type String) (Manager :type "RMusicManager Object Reference"))
  (switch `string` MarkerText
    (:`Bridge 1`
      (if (> (`self.GetHealthR`) 30.0)
        (`RMusicManager.GoBackToMarker` Manager "Chorus 1")))
    (:`Chorus 3`
      (if (> (`self.GetHealthR`) 20.0)
        (`RMusicManager.GoBackToMarker` Manager "Chorus 2")))
    (:`Bridge 2`
      (if (> (`self.GetHealthR`) 10.0)
        (`RMusicManager.GoBackToMarker` Manager "Chorus 3")))
    (:`Outro`
      (if (> (`self.GetHealthR`) 0.0)
        (`RMusicManager.GoBackToMarker` Manager "Chorus 4")))
    (:`End`
      (`/Engine/EditorBlueprintResources/StandardMacros.DoOnce` false
        (:`Completed`
          (bind _returnvalue (`|CreateWidget` "/Game/Blueprints/UI/BP_CompletedLevelScreen.BP_CompletedLevelScreen_C"))
          (`UserWidget.AddToViewport` _returnvalue 0))))))

(fn `UserConstructionScript`)