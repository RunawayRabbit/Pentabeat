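; BP_Pellet is a hostile pellet actor whose material flashes in time with the beat.
; On BeginPlay it creates a dynamic material instance from M_IMB_Yellow on the Quartz003 component and caches its default Color A and Color B.
; Every tick, both colors blend in HSV from FlashColor back to those defaults, driven by the clamped BeatProgress of its RBeatReaction component.
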(event `self.ReceiveBeginPlay`
  ;[1 1 1] Set Up Material Instance
  (bind _returnvalue (`PrimitiveComponent.CreateDynamicMaterialInstance` (`self.Quartz_003`) 0 "/Game/ColorPalettes/IMB/M_IMB_Yellow.M_IMB_Yellow" "None"))
  (bind _output_get (set `self.Material Instance` _returnvalue))
  (bind _returnvalue_2 (`MaterialInstanceDynamic.K2_GetVectorParameterValue` _output_get "Color A"))
  (set `self.Default Color A` _returnvalue_2)
  (bind _returnvalue_3 (`MaterialInstanceDynamic.K2_GetVectorParameterValue` _output_get "Color B"))
  (set `self.Default Color B` _returnvalue_3))

(event `self.ReceiveTick`
  (params (DeltaSeconds :type "Float (single-precision)"))
  (bind _returnvalue (`KismetMathLibrary.FClamp` (`RBeatReaction.BeatProgress` (`self.GetComponentByClass` "/Script/GP4_Team7.RBeatReaction"))))
  ;[1 1 1] Pulse Material At Low Lifespan
  (`|ExecutionSequence`
    (:`then_0`
      (`MaterialInstanceDynamic.SetVectorParameterValue` (`self.Material Instance`) "Color A" (`KismetMathLibrary.LinearColorLerpUsingHSV` (`self.Flash Color`) (`self.Default Color A`) _returnvalue)))
    (:`then_1`
      (`MaterialInstanceDynamic.SetVectorParameterValue` (`self.Material Instance`) "Color B" (`KismetMathLibrary.LinearColorLerpUsingHSV` (`self.Flash Color`) (`self.Default Color B`) _returnvalue)))))

(fn `UserConstructionScript`)