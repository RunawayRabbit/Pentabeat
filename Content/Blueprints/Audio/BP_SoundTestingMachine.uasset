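; BP_SoundTestingMachine is an audio test actor that lights three indicators in response to bassdrum, snare and hat tracks.
; It starts three audio components on BeginPlay and stores each one's envelope value through OnAudioSingleEnvelopeValue events.
; Every Tick, the Bassdrum, Snare and Hat functions compare those values to thresholds, lower for the hat, and swap each light's material between two test colors.
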(event `self.ReceiveBeginPlay`
  (`AudioComponent.Play` (`self.Audio 1`) 0.0)
  (`AudioComponent.Play` (`self.Audio 2`) 0.0)
  (`AudioComponent.Play` (`self.Audio 3`) 0.0))

(event `self.ReceiveTick`
  (params (DeltaSeconds :type "Float (single-precision)"))
  ;[1 1 1] Lights
  (`|ExecutionSequence`
    (:`then_0`
      (`self.Bassdrum`))
    (:`then_1`
      (`self.Snare`))
    (:`then_2`
      (`self.Hat`))))

(event `self.Audio 1.OnAudioSingleEnvelopeValue`
  (params (PlayingSoundWave :type "SoundWave Object Reference") (EnvelopeValue :type "Float (single-precision)"))
  ;[1 1 1] Envelopes
  (set `self.Bassdrum Envelope Value` EnvelopeValue))

(event `self.Audio 2.OnAudioSingleEnvelopeValue`
  (params (PlayingSoundWave :type "SoundWave Object Reference") (EnvelopeValue :type "Float (single-precision)"))
  ;[1 1 1] Envelopes
  (set `self.Snare Envelope Value` EnvelopeValue))

(event `self.Audio 3.OnAudioSingleEnvelopeValue`
  (params (PlayingSoundWave :type "SoundWave Object Reference") (EnvelopeValue :type "Float (single-precision)"))
  ;[1 1 1] Envelopes
  (set `self.Hat Envelope Value` EnvelopeValue))

(fn `Bassdrum`
  (bind _light_1 (`self.Light 1`))
  (if (>= (`self.Bassdrum Envelope Value`) 0.05)
    (`PrimitiveComponent.SetMaterial` _light_1 0 "/Game/Blueprints/Audio/M_TestingColorB.M_TestingColorB")
    (else
      (`PrimitiveComponent.SetMaterial` _light_1 0 "/Game/Blueprints/Audio/M_TestingColorA.M_TestingColorA"))))

(fn `Hat`
  (bind _light_3 (`self.Light 3`))
  (if (>= (`self.Hat Envelope Value`) 0.01)
    (`PrimitiveComponent.SetMaterial` _light_3 0 "/Game/Blueprints/Audio/M_TestingColorB.M_TestingColorB")
    (else
      (`PrimitiveComponent.SetMaterial` _light_3 0 "/Game/Blueprints/Audio/M_TestingColorA.M_TestingColorA"))))

(fn `Snare`
  (bind _light_2 (`self.Light 2`))
  (if (>= (`self.Snare Envelope Value`) 0.05)
    (`PrimitiveComponent.SetMaterial` _light_2 0 "/Game/Blueprints/Audio/M_TestingColorB.M_TestingColorB")
    (else
      (`PrimitiveComponent.SetMaterial` _light_2 0 "/Game/Blueprints/Audio/M_TestingColorA.M_TestingColorA"))))

(fn `UserConstructionScript`)