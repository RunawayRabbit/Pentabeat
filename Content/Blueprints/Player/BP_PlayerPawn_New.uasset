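; Player pawn that presents jumping, pellet shooting, damage invulnerability and death through sound, Niagara effects and UI.
; Component events drive jump flips, projectile spawning, and shield and orbiting-pellet visibility, with a beat-timed whoosh at three pellets.
; Invulnerability lerps dynamic material colors by beat progress, though a comment marks this broken.
; Death events show separate screens; pause input toggles a widget, whose creation code is disconnected.
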(event `OnBulletHit_Event_0` :!signature `self.OnBulletHit`
  (params (BulletLocation :type "Vector Structure"))
  (`NiagaraFunctionLibrary.SpawnSystemAtLocation` "/Game/ParticleEffects/Bullet/Explosion/N_BulletExplosion.N_BulletExplosion" BulletLocation))

(event `self.ReceiveBeginPlay`
  (`|ExecutionSequence`
    (:`then_0`
      (`self.SpawnFirstPellet`))
    (:`then_1`
      (add `self.OnDeath` (delegate `OnDeath_Event`))
      (add `self.OnFallingToDeath` (delegate `OnFallingToDeath_Event`))
      (add `self.OnBulletHit` (delegate `OnBulletHit_Event_0`)))
    (:`then_2`
      (add `self.OnInvulnerabilityStart` (delegate `OnInvulnerabilityStart_Event`))
      (add `self.OnInvulnerabilityEnd` (delegate `OnInvulnerability_End`))
      (`self.SetMaterialParameters`))
    (:`then_3`
      (`self.CreatePauseWidget`))
    (:`then_4`
      (`self.EnableInput` (`GameplayStatics.GetPlayerController` 0)))))

(event `OnDeath_Event`
  (`/Engine/EditorBlueprintResources/StandardMacros.DoOnce` false
    (:`Completed`
      (bind _returnvalue (`|CreateWidget` "/Game/Blueprints/UI/BP_DeathScreen.BP_DeathScreen_C"))
      (`UserWidget.AddToViewport` _returnvalue 0)
      (`GameplayStatics.PlaySoundAtLocation` "/Game/Sound/SFX/SoundCues/CueDeath.CueDeath" (0.0 0.0 0.0) (struct) 1.0 1.0 0.0 null null null))))

(event `OnFallingToDeath_Event`
  (`/Engine/EditorBlueprintResources/StandardMacros.DoOnce` false
    (:`Completed`
      (bind _returnvalue (`|CreateWidget` "/Game/Blueprints/UI/BP_FallingDeathScreen.BP_FallingDeathScreen_C"))
      (`UserWidget.AddToViewport` _returnvalue 0)
      (`GameplayStatics.PlaySoundAtLocation` "/Game/Sound/SFX/SoundCues/CueDeath.CueDeath" (0.0 0.0 0.0) (struct) 1.0 1.0 0.0 null null null))))

(event `OnInvulnerability_End` :!signature `self.OnInvulnerabilityEnd`
  (params (InvulnerabilityTimeRemaining :type "Float (double-precision)"))
  (set `self.ShouldFlash` false)
  (`|ExecutionSequence`
    (:`then_0`
      (`MaterialInstanceDynamic.SetVectorParameterValue` (`self.MeshMaterialInstance`) "Color A" (`self.Default Color A`)))
    (:`then_1`
      (`MaterialInstanceDynamic.SetVectorParameterValue` (`self.MeshMaterialInstance`) "Color B" (`self.Default Color B`)))))

(event `OnInvulnerabilityStart_Event` :!signature `self.OnInvulnerabilityStart`
  (params (InvulnerabilityTimeRemaining :type "Float (double-precision)"))
  (set `self.ShouldFlash` true))

(event `self.JumpingComponent.OnJumpStart`
  (bind _spinnyflip (`self.SpinnyFlip`))
  (bind _returnvalue (`SceneComponent.K2_GetComponentLocation` (`self.FeetLocation`)))
  (bind (_relativerotation_roll _relativerotation_pitch _relativerotation_yaw) (`KismetMathLibrary.BreakRotator` (`SceneComponent.RelativeRotation` _spinnyflip)))
  (`NiagaraFunctionLibrary.SpawnSystemAttached` "/Game/ParticleEffects/N_JumpingTrail_System.N_JumpingTrail_System" (`self.FeetLocation`) "None" _returnvalue (struct) "KeepWorldPosition" true)
  (`GameplayStatics.PlaySoundAtLocation` "/Game/Sound/SFX/SoundCues/CueJump.CueJump" _returnvalue (struct) 0.6 1.0 0.0 null null null)
  (bind _returnvalue_2 (`RJumpingComponent.GetJumpPercent` (`self.JumpingComponent`)))
  (bind (_direction _roll) (`Timeline|Timeline_0` :`NewTime` _returnvalue_2 :!via `PlayFromStart`)
    (:`Update`
      (`SceneComponent.K2_SetRelativeRotation` _spinnyflip (`KismetMathLibrary.MakeRotator` (* -1 _roll) _relativerotation_pitch _relativerotation_yaw) false false))))

(event `self.JumpingComponent.OnJumpLand`
  (bind _returnvalue (`SceneComponent.K2_GetComponentLocation` (`self.FeetLocation`)))
  (`NiagaraFunctionLibrary.SpawnSystemAtLocation` "/Game/ParticleEffects/N_Impact.N_Impact" _returnvalue (struct) (0.5 0.5 0.5))
  ;[1 1 1] LAND
  (`GameplayStatics.PlaySoundAtLocation` "/Game/Sound/SFX/SoundCues/CueLand.CueLand" _returnvalue (struct) 0.5 1.0 0.0 null null null))

(event `self.PelletComponent.OnPelletShoot`
  (params (PelletCount :type Integer) (Target :type "Actor Object Reference") (Damage :type "Float (single-precision)"))
  (bind _returnvalue (`|SpawnActorFromClass` "/Game/ParticleEffects/PelletAttack/BP_PelletProjectile.BP_PelletProjectile_C" (`KismetMathLibrary.MakeTransform` (`self.K2_GetActorLocation`)) "Undefined" "OverrideRootScale" null null))
  (`NiagaraComponent.SetVariableFloat` (`self.GetComponentByClass` _returnvalue "/Script/Niagara.NiagaraComponent") "Damage" Damage))

(event `self.PelletComponent.OnPelletAttemptPickupFull`
  (params (PelletCount :type Integer))
  ;[1 1 1] PICKUP FULL
  (`GameplayStatics.PlaySoundAtLocation` "/Game/Sound/SFX/SoundCues/CuePickupFull.CuePickupFull" (0.0 0.0 0.0) (struct) 2.0 1.0 0.0 null null null))

(event `self.PelletComponent.OnPelletBlock`
  (params (PelletCount :type Integer))
  (`GameplayStatics.PlaySoundAtLocation` "/Game/Sound/SFX/SoundCues/CueBlock.CueBlock" (0.0 0.0 0.0) (struct) 1.0 1.0 0.0 null null null))

(event `self.PelletComponent.OnPelletAttemptShootEmpty`
  (params (PelletCount :type Integer))
  ;[1 1 1] SHOOT EMPTY
  (`GameplayStatics.PlaySoundAtLocation` "/Game/Sound/SFX/SoundCues/CueShootEmpty.CueShootEmpty" (0.0 0.0 0.0) (struct) 1.0 1.0 0.0 null null null))

(event `InputAction|Pause` :paused true
  (params (Key :type "Key Structure"))
  (bind _pausewidget (`self.PauseWidget`))
  (:`Pressed`
    (if (`self.bIsDead`)
      _
      (elif (`self.IsPaused`)
        (`self.TogglePause` _pausewidget)
        (else
          (`self.TogglePause` _pausewidget true))))))

(event `self.PelletComponent.OnPelletCountChange`
  (params (PelletCount :type Integer))
  (`self.OnPelletCountChange` PelletCount)
  ;[1 1 1] PICKUP PELLET
  (`GameplayStatics.PlaySoundAtLocation` "/Game/Sound/SFX/SoundCues/CuePickup.CuePickup" (`self.K2_GetActorLocation`) (struct) 1.0 1.0 0.0 null null null))

(event `self.BeatReacton.React`
  (params (BeatNumber :type Integer) (Measure :type Integer) (Time :type Integer) (BPM :type Integer))
  (if (`self.Should Whoosh`)
    ;[1 1 1] WOOSH
    (`GameplayStatics.PlaySoundAtLocation` "/Game/Sound/SFX/SoundCues/CueWoosh.CueWoosh" (`self.K2_GetActorLocation`) (struct) 4.0 (`KismetMathLibrary.RandomFloatInRange` 0.97 1.03) 0.11 null null null)))

(event `self.ReceiveTick`
  (params (DeltaSeconds :type "Float (single-precision)"))
  (if (`self.ShouldFlash`)
    (`self.FlashMaterialOnInvulnerable`)))

(fn `CreatePauseWidget`)

(fn `FlashMaterialOnInvulnerable`
  (bind _returnvalue (`KismetMathLibrary.FClamp` (`RBeatReaction.BeatProgress` (`self.GetComponentByClass` "/Script/GP4_Team7.RBeatReaction"))))
  ;[1 1 1] Broken invulnerability flashes
  (`|ExecutionSequence`
    (:`then_0`
      (`MaterialInstanceDynamic.SetVectorParameterValue` (`self.MeshMaterialInstance`) "Color A" (`KismetMathLibrary.LinearColorLerpUsingHSV` (`self.Flash Color`) (`self.Default Color A`) _returnvalue)))
    (:`then_1`
      (`MaterialInstanceDynamic.SetVectorParameterValue` (`self.MeshMaterialInstance`) "Color B" (`KismetMathLibrary.LinearColorLerpUsingHSV` (`self.Flash Color`) (`self.Default Color B`) _returnvalue)))))

(fn `OnPelletCountChange`
  (params (Count :type Integer))
  (bind _onepellet_shield (`self.OnePellet_Shield`))
  (bind _twopellet_shield (`self.TwoPellet_Shield`))
  (bind _threepellet_shield (`self.ThreePellet_Shield`))
  (bind _pelletorbitingone (`self.PelletOrbitingOne`))
  (bind _pelletorbitingtwo (`self.PelletOrbitingTwo`))
  (bind _pelletorbitingthree (`self.PelletOrbitingThree`))
  (switch `int` Count
    (:`0`
      (`SceneComponent.SetVisibility` _onepellet_shield false false)
      (`SceneComponent.SetVisibility` _twopellet_shield false false)
      (`SceneComponent.SetVisibility` _threepellet_shield false false)
      (`SceneComponent.SetVisibility` _pelletorbitingone false false)
      (`SceneComponent.SetVisibility` _pelletorbitingtwo false false)
      (`SceneComponent.SetVisibility` _pelletorbitingthree false false)
      (set `self.Should Whoosh` false :!label _label))
    (:`1`
      (`SceneComponent.SetVisibility` _onepellet_shield true false)
      (`SceneComponent.SetVisibility` _twopellet_shield false false)
      (`SceneComponent.SetVisibility` _threepellet_shield false false)
      (`SceneComponent.SetVisibility` _pelletorbitingone true false)
      (`SceneComponent.SetVisibility` _pelletorbitingtwo false false)
      (`SceneComponent.SetVisibility` _pelletorbitingthree false false)
      (goto _label))
    (:`2`
      (`SceneComponent.SetVisibility` _onepellet_shield false false)
      (`SceneComponent.SetVisibility` _twopellet_shield true false)
      (`SceneComponent.SetVisibility` _threepellet_shield false false)
      (`SceneComponent.SetVisibility` _pelletorbitingone true false)
      (`SceneComponent.SetVisibility` _pelletorbitingtwo true false)
      (`SceneComponent.SetVisibility` _pelletorbitingthree false false)
      (goto _label))
    (:`3`
      (`SceneComponent.SetVisibility` _onepellet_shield false false)
      (`SceneComponent.SetVisibility` _twopellet_shield false false)
      (`SceneComponent.SetVisibility` _threepellet_shield true false)
      (`SceneComponent.SetVisibility` _pelletorbitingone true false)
      (`SceneComponent.SetVisibility` _pelletorbitingtwo true false)
      (`SceneComponent.SetVisibility` _pelletorbitingthree true false)
      (set `self.Should Whoosh` true))))

(fn `SetMaterialParameters`
  (bind _meshmaterialinstance (`self.MeshMaterialInstance`))
  (`|ExecutionSequence`
    (:`then_0`
      (bind _returnvalue (`PrimitiveComponent.CreateDynamicMaterialInstance` (`self.SkeletalMeshComponent`) 0 "/Game/ColorPalettes/IMB/M_IMB_Yellow.M_IMB_Yellow" "None"))
      (set `self.MeshMaterialInstance` _returnvalue))
    (:`then_1`
      (bind _returnvalue_2 (`MaterialInstanceDynamic.K2_GetVectorParameterValue` _meshmaterialinstance "Color A"))
      (set `self.Default Color A` _returnvalue_2))
    (:`then_2`
      (bind _returnvalue_3 (`MaterialInstanceDynamic.K2_GetVectorParameterValue` _meshmaterialinstance "Color B"))
      (set `self.Default Color B` _returnvalue_3))))

(fn `SpawnFirstPellet`
  (bind _returnvalue (`|SpawnActorFromClass` "/Game/Blueprints/Hostiles/BP_Pellet.BP_Pellet_C" (`KismetMathLibrary.MakeTransform` (.location (`self.GetTransform`)) (struct) (0.5 0.5 0.5)) "Undefined" "OverrideRootScale" null null))
  (`self.K2_AddActorLocalOffset` _returnvalue (* (`SceneComponent.GetForwardVector` (`self.RootComponent`)) 500.0) false false))

(fn `TogglePause`
  (params (InputPin :type "/Game/Blueprints/UI/BP_Pause Object Reference") (Enable :type Boolean))
  (`|ExecutionSequence`
    (:`then_0`
      (`Widget.SetIsEnabled` InputPin Enable))
    (:`then_1`
      (if Enable
        (`Widget.SetVisibility` InputPin "Visible")
        (else
          (`Widget.SetVisibility` InputPin "Hidden"))))
    (:`then_2`
      (set `self.IsPaused` Enable))
    (:`then_3`
      (`Widget.SetFocus` InputPin))
    (:`then_4`
      (`GameplayStatics.SetGamePaused` Enable))))

(fn `UserConstructionScript`)