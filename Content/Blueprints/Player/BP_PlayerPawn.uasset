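; Player pawn that jumps, collects and shoots pellets, spawns a starter pellet ahead of itself, and offers a return to menu on death.
; JumpingComponent events drive trail and impact effects, sounds and a timeline flip of the mesh pivot.
; PelletComponent events play feedback sounds, spawn projectiles that pass damage into their Niagara component, and switch shield visuals by pellet count.
; The three-pellet shield also enables randomized whoosh sounds on BeatReacton reactions.
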(event `self.ReceiveBeginPlay`
  (bind _returnvalue (`|SpawnActorFromClass` "/Game/Blueprints/Hostiles/BP_Pellet.BP_Pellet_C" (`KismetMathLibrary.MakeTransform` (.location (`self.GetTransform`)) (struct) (0.5 0.5 0.5)) "Undefined" "OverrideRootScale" null null))
  (`self.K2_AddActorLocalOffset` _returnvalue (* (`SceneComponent.GetForwardVector` (`self.RootComponent`)) 500.0) false false)
  (add `self.OnDeath` (delegate `OnDeath_Event`)))

(event `OnDeath_Event`
  (bind _returnvalue (`|CreateWidget` "/Game/Blueprints/UI/Widgets/BP_RestartText.BP_RestartText_C"))
  (`UserWidget.AddToViewport` _returnvalue 0))

(event `InputAction|GoBackToMenu`
  (params (Key :type "Key Structure"))
  (:`Pressed`
    (if (`self.bIsDead`)
      (`GameplayStatics.OpenLevelBySoftObjectPtr` "/Game/Level/Menus/L_MainMenu.L_MainMenu"))))

(event `self.JumpingComponent.OnJumpStart`
  (bind _skeletonmeshpivot (`self.SkeletonMeshPivot`))
  (bind _returnvalue (`SceneComponent.K2_GetComponentLocation` (`self.FeetLocation`)))
  (bind (_relativerotation_roll _relativerotation_pitch _relativerotation_yaw) (`KismetMathLibrary.BreakRotator` (`SceneComponent.RelativeRotation` _skeletonmeshpivot)))
  (`NiagaraFunctionLibrary.SpawnSystemAttached` "/Game/ParticleEffects/N_JumpingTrail_System.N_JumpingTrail_System" (`self.FeetLocation`) "None" _returnvalue (struct) "KeepWorldPosition" true)
  (`GameplayStatics.PlaySoundAtLocation` "/Game/Sound/SFX/SoundCues/CueJump.CueJump" _returnvalue (struct) 0.6 1.0 0.0 null null null)
  (bind _returnvalue_2 (`RJumpingComponent.GetJumpPercent` (`self.JumpingComponent`)))
  (bind (_direction _roll) (`Timeline|Da Epic Flip` :`NewTime` _returnvalue_2 :!via `PlayFromStart`)
    (:`Update`
      (`SceneComponent.K2_SetRelativeRotation` _skeletonmeshpivot (`KismetMathLibrary.MakeRotator` (* -1 _roll) _relativerotation_pitch _relativerotation_yaw) false false))))

(event `self.JumpingComponent.OnJumpLand`
  (bind _returnvalue (`SceneComponent.K2_GetComponentLocation` (`self.FeetLocation`)))
  (`NiagaraFunctionLibrary.SpawnSystemAtLocation` "/Game/ParticleEffects/N_Impact.N_Impact" _returnvalue (struct) (0.5 0.5 0.5))
  (`GameplayStatics.PlaySoundAtLocation` "/Game/Sound/SFX/SoundCues/CueLand.CueLand" _returnvalue (struct) 0.5 1.0 0.0 null null null))

(event `self.PelletComponent.OnPelletBlock`
  (params (PelletCount :type Integer))
  (`GameplayStatics.PlaySoundAtLocation` "/Game/Sound/SFX/SoundCues/CueBlock.CueBlock" (0.0 0.0 0.0) (struct) 1.0 1.0 0.0 null null null))

(event `self.PelletComponent.OnPelletShoot`
  (params (PelletCount :type Integer) (Target :type "Actor Object Reference") (Damage :type "Float (single-precision)"))
  (bind _returnvalue (`|SpawnActorFromClass` "/Game/ParticleEffects/PelletAttack/BP_PelletProjectile.BP_PelletProjectile_C" (`self.GetTransform`) "Undefined" "OverrideRootScale" null null))
  (`NiagaraComponent.SetVariableFloat` (`self.GetComponentByClass` _returnvalue "/Script/Niagara.NiagaraComponent") "Damage" Damage))

(event `self.PelletComponent.OnPelletAttemptPickupFull`
  (params (PelletCount :type Integer))
  (`GameplayStatics.PlaySoundAtLocation` "/Game/Sound/SFX/SoundCues/CuePickupFull.CuePickupFull" (0.0 0.0 0.0) (struct) 2.0 1.0 0.0 null null null))

(event `self.PelletComponent.OnPelletAttemptShootEmpty`
  (params (PelletCount :type Integer))
  (`GameplayStatics.PlaySoundAtLocation` "/Game/Sound/SFX/SoundCues/CueShootEmpty.CueShootEmpty" (0.0 0.0 0.0) (struct) 1.0 1.0 0.0 null null null))

(event `self.PelletComponent.OnPelletCountChange`
  (params (PelletCount :type Integer))
  (`self.OnPelletCountChange` PelletCount)
  (`GameplayStatics.PlaySoundAtLocation` "/Game/Sound/SFX/SoundCues/CuePickup.CuePickup" (0.0 0.0 0.0) (struct) 1.0 1.0 0.0 null null null))

(event `self.BeatReacton.React`
  (params (BeatNumber :type Integer) (Measure :type Integer) (Time :type Integer) (BPM :type Integer))
  (if (`self.ShouldWoosh`)
    (`GameplayStatics.PlaySoundAtLocation` (select `bool` (`KismetMathLibrary.RandomBool`) :`false` "/Game/Sound/SFX/Whoosh_Electric_00.Whoosh_Electric_00" :`true` "/Game/Sound/SFX/Whoosh_Electric_02.Whoosh_Electric_02" :!type "SoundBase Object Reference") (`self.K2_GetActorLocation`) (struct) 10.0 (`KismetMathLibrary.RandomFloatInRange` 0.97 1.03) 0.11 null null null)))

(fn `OnPelletCountChange`
  (params (Selection :type Integer))
  (switch `int` Selection
    (:`0`
      (`SceneComponent.SetVisibility` (`self.OnePellet_Shield`) false false)
      (`SceneComponent.SetVisibility` (`self.TwoPellet_Shield`) false false)
      (`SceneComponent.SetVisibility` (`self.ThreePellet_Shield`) false false)
      (set `self.ShouldWoosh` false :!label _label))
    (:`1`
      (`SceneComponent.SetVisibility` (`self.OnePellet_Shield`) true false)
      (`SceneComponent.SetVisibility` (`self.TwoPellet_Shield`) false false)
      (`SceneComponent.SetVisibility` (`self.ThreePellet_Shield`) false false)
      (goto _label))
    (:`2`
      (`SceneComponent.SetVisibility` (`self.OnePellet_Shield`) false false)
      (`SceneComponent.SetVisibility` (`self.TwoPellet_Shield`) true false)
      (`SceneComponent.SetVisibility` (`self.ThreePellet_Shield`) false false)
      (goto _label))
    (:`3`
      (`SceneComponent.SetVisibility` (`self.OnePellet_Shield`) false false)
      (`SceneComponent.SetVisibility` (`self.TwoPellet_Shield`) false false)
      (`SceneComponent.SetVisibility` (`self.ThreePellet_Shield`) true false)
      (set `self.ShouldWoosh` true))))

(fn `UserConstructionScript`)